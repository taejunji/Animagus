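; BP_SmartC is an unfinished AI perception Blueprint meant to react to sight, hearing and damage stimuli.
; CanSenseActor maps a sense enum to its AISense class and returns the first matching stimulus's success state, though its Actor input is unused.
; A per-actor loop prints sensed results and passes sightings to an empty HandleSenseSight.
; That loop is disconnected from OnPerceptionUpdated, so it never runs.
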(event `self.AIPerception.OnPerceptionUpdated`
  (params (UpdatedActors :type "Array of Actor Object Reference (by ref)")))

(fn `Can Sense Actor`
  (params (Actor :type "Actor Object Reference") (Sense :type "/Game/WorkFolder/AI/Data/E_AI_Sense Enum" :default "NewEnumerator0"))
  (returns (Sensed :type Boolean) (Stimulus :type "AIStimulus Structure"))
  (bind _info (`AIPerceptionComponent.GetActorsPerception` (`self.AIPerception`) null))
  (for _array_element (`.LastSensedStimuli` (break `ActorPerceptionBlueprintInfo` _info))
    (bind _returnvalue (`AIPerceptionSystem.GetSenseClassForStimulus` _array_element))
    (if (== _returnvalue (select `/Game/WorkFolder/AI/Data/E_AI_Sense` Sense :`NewEnumerator0` "/Script/AIModule.AISense_Sight" :`NewEnumerator1` "/Script/AIModule.AISense_Hearing" :`NewEnumerator2` "/Script/AIModule.AISense_Damage" :!type "Object Class Reference"))
      (return (`.bSuccessfullySensed` (break `AIStimulus` _array_element)) _array_element))))

(fn `Handle Sense Sight`
  (params (Actor :type "Actor Object Reference")))

(fn `UserConstructionScript`)