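; BP_AIPlayer is an AI player character that shows floating name, power level and damage indicator widgets.
; Every tick it rotates the damage widget toward the local camera, and the name widget too while the character is alive.
; Custom events pass damage values to WBP_DmgIndicator and write the BaseCharacter name and level into WBP_Name, switching to a restyled "MAX" label above the level cap.
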(event `self.ReceiveTick`
  (params (DeltaSeconds :type "Float (single-precision)"))
  (bind _damge_indicator_widget (`self.Damge Indicator Widget`))
  (bind _name_widget (`self.Name Widget`))
  (`SceneComponent.K2_SetWorldRotation` _damge_indicator_widget (`KismetMathLibrary.FindLookAtRotation` (`SceneComponent.K2_GetComponentLocation` _damge_indicator_widget) (`self.K2_GetActorLocation` (`GameplayStatics.GetPlayerCameraManager` 0))) false false)
  (bind _asbase_character (cast `BaseCharacter` self))
  (if (not (`BaseCharacter.is_dead` _asbase_character))
    (`SceneComponent.K2_SetWorldRotation` _name_widget (`KismetMathLibrary.FindLookAtRotation` (`SceneComponent.K2_GetComponentLocation` _name_widget) (`self.K2_GetActorLocation` (`GameplayStatics.GetPlayerCameraManager` 0))) false false)))

(event `self.ShowDmgIndicator`
  (params (ActualDmg :type "Float (single-precision)"))
  (bind _aswbp_dmg_indicator (cast `/Game/WorkFolder/Bluprints/Ui/WBP_DmgIndicator` (`WidgetComponent.GetWidget` (`self.Damge Indicator Widget`))))
  (`/Game/WorkFolder/Bluprints/Ui/WBP_DmgIndicator.Custom Apply Damage` _aswbp_dmg_indicator (`KismetTextLibrary.Conv_DoubleToText` ActualDmg "HalfToEven")))

(event `self.SetCharacterNameWidget`
  (bind _asbase_character (cast `BaseCharacter` self))
  (bind _aswbp_name (cast `/Game/WorkFolder/Bluprints/Ui/WBP_Name` (`WidgetComponent.GetWidget` (`self.Name Widget`))))
  (`TextBlock.SetText` (`/Game/WorkFolder/Bluprints/Ui/WBP_Name.NameText` _aswbp_name) (`KismetTextLibrary.Conv_StringToText` (`BaseCharacter.character_name` _asbase_character))))

(event `self.SetPowerLevelWidget`
  (params (level :type Integer))
  (bind _aswbp_name (cast `/Game/WorkFolder/Bluprints/Ui/WBP_Name` (`WidgetComponent.GetWidget` (`self.Name Widget`))))
  (if (<= level 14)
    (bind _leveltext (`/Game/WorkFolder/Bluprints/Ui/WBP_Name.LevelText` _aswbp_name))
    (`TextBlock.SetText` _leveltext (`KismetTextLibrary.Conv_IntToText` level))
    (else
      (set `TextBlock.Font` (make `SlateFontInfo` "/Game/CuteUIKit2/UI/Font/CAFE24SSURROUND-V2_0_Font.CAFE24SSURROUND-V2_0_Font" null (make `FontOutlineSettings` 3) "None" 20.0) _leveltext)
      (`TextBlock.SetText` _leveltext "MAX"))))

(fn `UserConstructionScript`)