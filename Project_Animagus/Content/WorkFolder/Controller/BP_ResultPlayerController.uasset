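; BP_ResultPlayerController is a player controller that stages the result level's scene for a win or a loss.
; Setter functions store references to level actors and four losing characters, and SetBluePrintLevel branches on IsWin.
; A win brightens the light, applies a day sky and plays the win sequence at reduced speed.
; A loss repositions the main camera, dims the light, applies a night sky and reveals the losing characters.
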(event `self.SetBluePrintLevel`
  (params (isWin :type Boolean))
  (if isWin
    (`self.SetWin`)
    (else
      (`self.SetLose`))))

(fn `SetLevelActors`
  (params (Light :type "/Game/WorkFolder/Bluprints/Rendering/BP_DirectionalLight Object Reference") (Sky :type "/Game/WorkFolder/Bluprints/Rendering/BP_SkySphere Object Reference") (Cloud :type "VolumetricCloud Object Reference") (Camera :type "CameraActor Object Reference") (CineCamera :type "CineCameraActor Object Reference") (WinSequence :type "LevelSequenceActor Object Reference"))
  (set `self.Light` Light)
  (set `self.SkySphere` Sky)
  (set `self.Cloud` Cloud)
  (set `self.MainCamera` Camera)
  (set `self.Cine Camera` CineCamera)
  (set `self.Win Sequence` WinSequence))

(fn `SetLevelChracters`
  (params (Lose1 :type "/Game/WorkFolder/Bluprints/Actor/BP_LoginCharacter Object Reference") (Lose2 :type "/Game/WorkFolder/Bluprints/Actor/BP_LoginCharacter Object Reference") (Lose3 :type "/Game/WorkFolder/Bluprints/Actor/BP_LoginCharacter Object Reference") (Lose4 :type "/Game/WorkFolder/Bluprints/Actor/BP_LoginCharacter Object Reference"))
  (set `self.Lose 1` Lose1)
  (set `self.Lose 2` Lose2)
  (set `self.Lose 3` Lose3)
  (set `self.Lose 4` Lose4))

(fn `SetLose`
  (`SceneComponent.K2_SetWorldTransform` (`CameraActor.CameraComponent` (`self.MainCamera`)) (`KismetMathLibrary.MakeTransform` (-115.0 -25.0 -25.0) (struct :`Pitch` 8.981291 :`Yaw` 20.722861)) false false)
  (`LightComponent.SetIntensity` (`Light.LightComponent` (`self.Light`)) 2.0)
  (`PrimitiveComponent.SetMaterial` (`StaticMeshActor.StaticMeshComponent` (`self.SkySphere`)) 0 "/Game/QMS_Cartoon_Skybox_Free/Material_Instances/MI_Sky0003_Night.MI_Sky0003_Night")
  (`SceneComponent.SetVisibility` (`Character.Mesh` (`self.Lose 1`)) true false)
  (`SceneComponent.SetVisibility` (`Character.Mesh` (`self.Lose 2`)) true false)
  (`SceneComponent.SetVisibility` (`Character.Mesh` (`self.Lose 3`)) true false)
  (`SceneComponent.SetVisibility` (`Character.Mesh` (`self.Lose 4`)) true false))

(fn `SetWin`
  (bind _sequenceplayer (`LevelSequenceActor.SequencePlayer` (`self.Win Sequence`)))
  (`LightComponent.SetIntensity` (`Light.LightComponent` (`self.Light`)) 4.0)
  (`PrimitiveComponent.SetMaterial` (`StaticMeshActor.StaticMeshComponent` (`self.SkySphere`)) 0 "/Game/QMS_Cartoon_Skybox_Free/Material_Instances/MI_Sky0005_DaySun.MI_Sky0005_DaySun")
  (`MovieSceneSequencePlayer.SetPlayRate` _sequenceplayer 0.7)
  (`MovieSceneSequencePlayer.Play` _sequenceplayer))

(fn `UserConstructionScript`)