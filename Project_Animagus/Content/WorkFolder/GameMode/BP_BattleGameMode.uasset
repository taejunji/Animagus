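; Battle game mode that restyles the level's lighting, sky and ambient effects for each of three rounds (0–2).
; SetLevelObject stores the light, sky and cloud references, and SetBluePrintLevel passes the current round to the Set functions.
; These adjust the light, swap the sky material and toggle all wind-line and firefly effects, with fireflies replacing wind lines in round 2.
; SetCloud is an empty stub.
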(event `self.ReceiveBeginPlay`)

(event `self.SetBluePrintLevel`
  (params (CurRound :type Integer))
  (`self.SetLight` CurRound)
  (`self.SetCloud` CurRound)
  (`self.SetSky` CurRound)
  (`self.SetObjects` CurRound))

(fn `SetCloud`
  (params (CurrentRound :type Integer)))

(fn `SetLevelObject`
  (params (inputLight :type "/Game/WorkFolder/Bluprints/Rendering/BP_DirectionalLight Object Reference") (inputSky :type "/Game/WorkFolder/Bluprints/Rendering/BP_SkySphere Object Reference") (inputCloud :type "VolumetricCloud Object Reference"))
  (set `self.Light` inputLight)
  (set `self.Sky` inputSky)
  (set `self.Cloud` inputCloud))

(fn `SetLight`
  (params (CurrentRound :type Integer))
  (bind _light (`self.Light`))
  (bind _lightcomponent (`Light.LightComponent` (`self.Light`)))
  (if (== CurrentRound 0)
    (`LightComponent.SetIntensity` _lightcomponent 4.0)
    (`self.K2_SetActorRotation` _light (struct :`Pitch` -37.535793 :`Yaw` -176.876207 :`Roll` -138.894577) false)
    (elif (== CurrentRound 1)
      (`LightComponent.SetIntensity` _lightcomponent 40.0)
      (`self.K2_SetActorRotation` _light (struct :`Pitch` -12.242162 :`Yaw` -176.8152 :`Roll` -139.167736) false)
      (`LightComponent.SetLightColor` _lightcomponent (make `LinearColor` 1.0 0.03689) true)
      (elif (== CurrentRound 2)
        (`LightComponent.SetIntensity` _lightcomponent 0.3)
        (`self.K2_SetActorRotation` _light (struct :`Pitch` -36.357901 :`Yaw` -143.858152 :`Roll` -97.853333) false)))))

(fn `SetObjects`
  (params (`Current Round` :type Integer))
  (if (== `Current Round` 0)
    (bind _outactors (`GameplayStatics.GetAllActorsOfClass` "/Game/WorkFolder/Bluprints/Rendering/BP_WindLine.BP_WindLine_C"))
    (for _array_element _outactors
      (`SceneComponent.SetVisibility` (`Emitter.ParticleSystemComponent` _array_element) true false)
      (bind _outactors_2 (`GameplayStatics.GetAllActorsOfClass` "/Game/WorkFolder/Bluprints/Rendering/BP_Firefly.BP_Firefly_C" :!label _label))
      (for _array_element_2 _outactors_2
        (`SceneComponent.SetVisibility` (`NiagaraActor.NiagaraComponent` _array_element_2) false false)))
    (goto _label)
    (elif (== `Current Round` 1)
      (bind _outactors_3 (`GameplayStatics.GetAllActorsOfClass` "/Game/WorkFolder/Bluprints/Rendering/BP_WindLine.BP_WindLine_C"))
      (for _array_element_3 _outactors_3
        (`SceneComponent.SetVisibility` (`Emitter.ParticleSystemComponent` _array_element_3) true false)
        (bind _outactors_4 (`GameplayStatics.GetAllActorsOfClass` "/Game/WorkFolder/Bluprints/Rendering/BP_Firefly.BP_Firefly_C" :!label _label_2))
        (for _array_element_4 _outactors_4
          (`SceneComponent.SetVisibility` (`NiagaraActor.NiagaraComponent` _array_element_4) false false)))
      (goto _label_2)
      (elif (== `Current Round` 2)
        (bind _outactors_5 (`GameplayStatics.GetAllActorsOfClass` "/Game/WorkFolder/Bluprints/Rendering/BP_WindLine.BP_WindLine_C"))
        (for _array_element_5 _outactors_5
          (`SceneComponent.SetVisibility` (`Emitter.ParticleSystemComponent` _array_element_5) false false)
          (bind _outactors_6 (`GameplayStatics.GetAllActorsOfClass` "/Game/WorkFolder/Bluprints/Rendering/BP_Firefly.BP_Firefly_C" :!label _label_3))
          (for _array_element_6 _outactors_6
            (`SceneComponent.SetVisibility` (`NiagaraActor.NiagaraComponent` _array_element_6) true false)))
        (goto _label_3)))))

(fn `SetSky`
  (params (CurrentRound :type Integer))
  (bind _staticmeshcomponent (`StaticMeshActor.StaticMeshComponent` (`self.Sky`)))
  (if (== CurrentRound 0)
    (`PrimitiveComponent.SetMaterial` _staticmeshcomponent 0 "/Game/QMS_Cartoon_Skybox_Free/Material_Instances/MI_Sky0005_DaySun.MI_Sky0005_DaySun")
    (elif (== CurrentRound 1)
      (`PrimitiveComponent.SetMaterial` _staticmeshcomponent 0 "/Game/QMS_Cartoon_Skybox_Free/Material_Instances/MI_Sky0006_NightMoon.MI_Sky0006_NightMoon")
      (elif (== CurrentRound 2)
        (`PrimitiveComponent.SetMaterial` _staticmeshcomponent 0 "/Game/QMS_Cartoon_Skybox_Free/Material_Instances/MI_Sky0003_Night.MI_Sky0003_Night")))))

(fn `UserConstructionScript`)