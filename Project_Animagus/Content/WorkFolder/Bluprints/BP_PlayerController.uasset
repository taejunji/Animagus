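; Player controller that turns Enhanced Input actions into look, movement and jump for the possessed pawn.
; BeginPlay adds the IMC_Player mapping context to player 0's input subsystem.
; IA_Rotate feeds yaw and pitch, while IA_Move drives movement along the full control rotation's forward and right vectors, without flattening pitch.
; IA_Jump calls Jump only when the controlled pawn is a Character.
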(event `self.ReceiveBeginPlay`
  (`EnhancedInputSubsystemInterface.AddMappingContext` (pcsubsystem `EnhancedInputLocalPlayerSubsystem` (`GameplayStatics.GetPlayerController` 0)) "/Game/WorkFolder/Controller/IMC_Player.IMC_Player" 0 (struct)))

(event `EnhancedInput|/Game/WorkFolder/Controller/IA_Rotate`
  (params (ActionValue :type "Vector2D Structure") (ElapsedSeconds :type "Float (double-precision)") (TriggeredSeconds :type "Float (double-precision)") (InputAction :type "InputAction Object Reference" :default "/Game/WorkFolder/Controller/IA_Rotate.IA_Rotate"))
  (:`Triggered`
    (`self.AddYawInput` ActionValue_X)
    (`self.AddPitchInput` ActionValue_Y)))

(event `EnhancedInput|/Game/WorkFolder/Controller/IA_Move`
  (params (ActionValue :type "Vector2D Structure") (ElapsedSeconds :type "Float (double-precision)") (TriggeredSeconds :type "Float (double-precision)") (InputAction :type "InputAction Object Reference" :default "/Game/WorkFolder/Controller/IA_Move.IA_Move"))
  (bind _returnvalue (`self.K2_GetPawn`))
  (bind _returnvalue_2 (`self.GetControlRotation`))
  (:`Triggered`
    (`Pawn.AddMovementInput` _returnvalue (`KismetMathLibrary.GetForwardVector` _returnvalue_2) ActionValue_X false)
    (`Pawn.AddMovementInput` _returnvalue (`KismetMathLibrary.GetRightVector` _returnvalue_2) ActionValue_Y false)))

(event `EnhancedInput|/Game/WorkFolder/Controller/IA_Jump`
  (params (ActionValue :type Boolean) (ElapsedSeconds :type "Float (double-precision)") (TriggeredSeconds :type "Float (double-precision)") (InputAction :type "InputAction Object Reference" :default "/Game/WorkFolder/Controller/IA_Jump.IA_Jump"))
  (:`Triggered`
    (bind `_as캐릭터` (cast `Character` (`self.K2_GetPawn`)))
    (`Character.Jump` `_as캐릭터`)))

(fn `UserConstructionScript`)