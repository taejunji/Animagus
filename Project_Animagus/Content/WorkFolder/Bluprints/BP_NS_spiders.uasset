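; BP_NS_spiders is an actor that drives a Niagara swarm effect, apparently spiders, that switches into attack when something enters its Box.
; Any overlapping actor becomes AttackTarget and turns on the User.Attack parameter of the NiagaraRats component; any end overlap clears both.
; While the target is valid, Tick feeds User.Player with player 0's location, regardless of which actor triggered the overlap.
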(event `self.ReceiveTick`
  (params (DeltaSeconds :type "Float (single-precision)"))
  (`/Engine/EditorBlueprintResources/StandardMacros.IsValid` (`self.Attack target`)
    (:`Is Valid`
      (`NiagaraComponent.SetVariableVec3` (`self.NiagaraRats`) "User.Player" (`self.K2_GetActorLocation` (`GameplayStatics.GetPlayerCharacter` 0))))))

(event `self.Box.OnComponentBeginOverlap`
  (params (OverlappedComponent :type "PrimitiveComponent Object Reference") (OtherActor :type "Actor Object Reference") (OtherComp :type "PrimitiveComponent Object Reference") (OtherBodyIndex :type Integer) (bFromSweep :type Boolean) (SweepResult :type "HitResult Structure (by ref)"))
  (set `self.Attack target` OtherActor)
  (`NiagaraComponent.SetVariableFloat` (`self.NiagaraRats`) "User.Attack" 1.0))

(event `self.Box.OnComponentEndOverlap`
  (params (OverlappedComponent :type "PrimitiveComponent Object Reference") (OtherActor :type "Actor Object Reference") (OtherComp :type "PrimitiveComponent Object Reference") (OtherBodyIndex :type Integer))
  (set `self.Attack target` null)
  (`NiagaraComponent.SetVariableFloat` (`self.NiagaraRats`) "User.Attack" 0.0))

(fn `UserConstructionScript`)