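; BP_MonsterController is a simple AI controller for a monster that runs the BT_Monster behavior tree when it possesses a pawn.
; On BeginPlay it records the controlled pawn's location in StartLoc, which this graph never reads.
; A disconnected chain that would push the character forward and make it jump never runs, and Tick is empty.
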(event `self.ReceivePossess`
  (params (PossessedPawn :type "Pawn Object Reference"))
  (`self.RunBehaviorTree` "/Game/WorkFolder/Bluprints/AISimple/BT_Monster.BT_Monster"))

(event `self.ReceiveTick`
  (params (DeltaSeconds :type "Float (single-precision)")))

(event `self.ReceiveBeginPlay`
  (set `self.StartLoc` (`self.K2_GetActorLocation` (`self.K2_GetPawn`))))

(event `Key|Six`
  (params (Key :type "Key Structure")))

(fn `UserConstructionScript`)